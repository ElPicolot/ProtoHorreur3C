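; Barrel (Tonneau) actor whose cylinder moves vertically according to flags on the first-person character.
; Each Tick, while DeplaCylindre is set, Testeau plays or reverses a timeline that lerps Z from its starting height by DistanceDiff.
; The start height is captured in world space at BeginPlay but applied as relative location.
; Interaction only prints debug text, and older movement and rotation nodes remain disconnected.
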(event `self.ReceiveTick`
  (params (DeltaSeconds :type "Float (single-precision)"))
  (bind (_returnvalue_x _returnvalue_y _returnvalue_z) (`KismetMathLibrary.BreakVector` (`SceneComponent.K2_GetComponentLocation` (`self.Cylinder`))))
  (`KismetSystemLibrary.PrintString` (`KismetStringLibrary.Conv_DoubleToString` _returnvalue_z) true true (struct :`R` 1.0 :`B` 0.372698 :`A` 1.0))
  (bind _asbp_first_person_character (cast `/Game/FirstPerson/Blueprints/BP_FirstPersonCharacter` (`GameplayStatics.GetPlayerCharacter` 0)))
  (`KismetSystemLibrary.PrintString` "interagit")
  (if (`/Game/FirstPerson/Blueprints/BP_FirstPersonCharacter.deplaCylindre` _asbp_first_person_character)
    (`KismetSystemLibrary.PrintString` "interagitCylind")
    (if (`/Game/FirstPerson/Blueprints/BP_FirstPersonCharacter.testeau` _asbp_first_person_character)
      (`TimelineComponent.SetPlayRate` (`self.Timeline_0`) (`self.Movement Duration`))
      (bind (_direction _newtrack_0) (`Timeline|Timeline_0` :!label _label)
        (:`Update`
          (`SceneComponent.K2_SetRelativeLocation` (`self.Cylinder`) (`KismetMathLibrary.MakeVector` 0.0 0.0 (`KismetMathLibrary.Lerp` (`self.hauteur`) (+ (`self.hauteur`) (`self.distanceDiff`)) _newtrack_0)) false false)))
      (else
        (goto _label :!via `Reverse`)))))

(event `self.ReceiveBeginPlay`
  (bind (_returnvalue_x _returnvalue_y _returnvalue_z) (`KismetMathLibrary.BreakVector` (`SceneComponent.K2_GetComponentLocation` (`self.Cylinder`))))
  (set `self.hauteur` _returnvalue_z)
  (set `self.Return Value Z` _returnvalue_z))

(event `self.Interaction`
  (`KismetSystemLibrary.PrintString` "avantinteragit" true true (struct :`R` 1.0 :`B` 0.372698 :`A` 1.0)))

(fn `UserConstructionScript`)