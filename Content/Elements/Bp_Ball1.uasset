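; Bp_Ball1 is an actor that makes the first-person player's flashlight flicker according to its distance from the player, with debug prints.
; Tick clears Danger; below 300 units it stops there, otherwise a 0.3-second Delay and FlipFlop toggle flashlight intensity and LumBas.
; The middle range check compares constant 0 to 500, so it always passes and the 700-unit band that sets Danger is unreachable.
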(event `self.ReceiveTick`
  (params (DeltaSeconds :type "Float (single-precision)"))
  (bind _returnvalue (`KismetMathLibrary.Round` (`self.GetDistanceTo` (`GameplayStatics.GetPlayerCharacter` 0))))
  (if (and (not (`self.LumBas`)) (`self.Danger`))
    (bind _asbp_first_person_character (cast `/Game/FirstPerson/Blueprints/BP_FirstPersonCharacter` (`GameplayStatics.GetPlayerCharacter` 0)))
    (`LightComponent.SetIntensity` (`/Game/FirstPerson/Blueprints/BP_FirstPersonCharacter.Flashlight` _asbp_first_person_character) 50000.0)
    (else
      (`KismetSystemLibrary.PrintString` "FALSE Intense" true true (struct :`G` 1.0 :`B` 0.217085 :`A` 1.0))
      (if (< _returnvalue 300)
        (`KismetSystemLibrary.PrintString` "danger3" true true (struct :`R` 1.0 :`G` 0.073941 :`A` 1.0))
        (set `self.Danger` false)
        (elif (< 0 500)
          (`KismetSystemLibrary.PrintString` "danger2" true true (struct :`R` 1.0 :`G` 0.479777 :`A` 1.0))
          (set `self.Danger` false)
          (if (`self.Danger`) :!label _label
            (bind _asbp_first_person_character_2 (cast `/Game/FirstPerson/Blueprints/BP_FirstPersonCharacter` (`GameplayStatics.GetPlayerCharacter` 0)))
            (`LightComponent.SetLightColor` (`/Game/FirstPerson/Blueprints/BP_FirstPersonCharacter.Flashlight` _asbp_first_person_character_2) (struct :`R` 1.0 :`G` 1.0 :`B` 1.0 :`A` 1.0) true)
            (`KismetSystemLibrary.PrintString` "colordangert")
            (else
              (bind _asbp_first_person_character_3 (cast `/Game/FirstPerson/Blueprints/BP_FirstPersonCharacter` (`GameplayStatics.GetPlayerCharacter` 0)))
              (`KismetSystemLibrary.Delay` 0.3)
              (`/Engine/EditorBlueprintResources/StandardMacros.FlipFlop`
                (:`A`
                  (bind _flashlight (`/Game/FirstPerson/Blueprints/BP_FirstPersonCharacter.Flashlight` _asbp_first_person_character_3))
                  (`LightComponent.SetIntensity` _flashlight 0.0)
                  (`KismetSystemLibrary.PrintString` "color intense")
                  (set `self.LumBas` false))
                (:`B`
                  (`LightComponent.SetIntensity` _flashlight 50000.0)
                  (`KismetSystemLibrary.PrintString` "color clean")
                  (set `self.LumBas` true)))))
          (elif (< _returnvalue 700)
            (`KismetSystemLibrary.PrintString` "danger1" true true (struct :`G` 1.0 :`B` 0.194704 :`A` 1.0))
            (set `self.Danger` true)
            (goto _label)))))))

(fn `UserConstructionScript`)