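; Boss walking enemy Blueprint that begins chasing the player when it sees a pawn through PawnSensing.
; OnSeePawn sets IsSeeingPlayer and calls FollowPlayer, which clears CanAttack, prints a debug string and issues AIMoveTo toward player character 0.
; The attack check on successful arrival is an empty stub, and nothing in the graph resets IsSeeingPlayer.
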(event `self.PawnSensing.OnSeePawn`
  (params (Pawn :type "Pawn Object Reference"))
  (set `self.isSeeingPlayer` true)
  (`self.FollowPlayer`))

(event `FollowPlayer`
  (set `self.canAttack` false)
  (if (`self.isSeeingPlayer`)
    (`KismetSystemLibrary.PrintString` "true follow")
    (`|AIMoveTo` self (0.0 0.0 0.0) (`GameplayStatics.GetPlayerCharacter` 0)
      (:`OnSuccess`
        (if (`self.canAttack`)
          _)))))

(fn `UserConstructionScript`)