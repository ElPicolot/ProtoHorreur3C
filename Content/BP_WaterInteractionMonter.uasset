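; Water-interaction actor that grows vertically while the first-person character is inside its Box trigger.
; BeginPlay stores the starting location and scale; only the scale is used afterwards.
; Overlap plays CubeTimeline at a rate set by ScalingDurationLength, lerping actor Z scale toward six times the original, and leaving reverses it.
; Debug prints trace each stage, and unconnected mesh rotation, scale and location experiments remain in the graph.
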(event `self.ReceiveBeginPlay`
  (`KismetSystemLibrary.PrintString` "store Variables point")
  (`self.StoreValuesPoints`))

(event `self.Box.OnComponentBeginOverlap`
  (params (OverlappedComponent :type "PrimitiveComponent Object Reference") (OtherActor :type "Actor Object Reference") (OtherComp :type "PrimitiveComponent Object Reference") (OtherBodyIndex :type Integer) (bFromSweep :type Boolean) (SweepResult :type "HitResult Structure (by ref)"))
  (bind (_startscale_x _startscale_y _startscale_z) (`KismetMathLibrary.BreakVector` (`self.StartScale`)))
  (`KismetSystemLibrary.PrintString` "overlap")
  (cast `/Game/FirstPerson/Blueprints/BP_FirstPersonCharacter` OtherActor)
  (`TimelineComponent.SetPlayRate` (`self.CubeTimeline`) (`self.Scaling Duration Length`))
  (bind (_direction _alpha _scaletime) (`Timeline|CubeTimeline` :!label _label)
    (:`Update`
      (`KismetSystemLibrary.PrintString` (`KismetStringLibrary.Conv_DoubleToString` _alpha) true true (struct :`R` 1.0 :`G` 0.659101 :`A` 1.0))
      (`KismetSystemLibrary.PrintString` (`KismetStringLibrary.Conv_DoubleToString` _scaletime) true true (struct :`R` 0.289569 :`B` 1.0 :`A` 1.0))
      (bind (_returnvalue_x _returnvalue_y _returnvalue_z) (`KismetMathLibrary.BreakVector` (`KismetMathLibrary.VLerp` (`self.StartScale`) (`KismetMathLibrary.MakeVector` 0.0 0.0 (* _startscale_z 6.0)) _scaletime)))
      (`self.SetActorScale3D` (`KismetMathLibrary.MakeVector` _startscale_x _startscale_y _returnvalue_z))
      (`KismetSystemLibrary.PrintString` (`KismetStringLibrary.Conv_DoubleToString` _returnvalue_z) true true (struct :`R` 0.561444 :`G` 1.0 :`B` 0.083097 :`A` 1.0)))))

(event `self.Box.OnComponentEndOverlap`
  (params (OverlappedComponent :type "PrimitiveComponent Object Reference") (OtherActor :type "Actor Object Reference") (OtherComp :type "PrimitiveComponent Object Reference") (OtherBodyIndex :type Integer))
  (`KismetSystemLibrary.PrintString` "NBo_overlap")
  (cast `/Game/FirstPerson/Blueprints/BP_FirstPersonCharacter` OtherActor)
  (goto _label :!via `Reverse`))

(fn `StoreValuesPoints`
  (set `self.StartLocation` (`self.K2_GetActorLocation`))
  (set `self.StartScale` (`self.GetActorScale3D`))
  (`KismetSystemLibrary.PrintString` (`KismetStringLibrary.Conv_VectorToString` (`self.StartLocation`)) true true (struct :`R` 1.0 :`B` 0.363356 :`A` 1.0))
  (`KismetSystemLibrary.PrintString` (`KismetStringLibrary.Conv_VectorToString` (`self.StartScale`)) true true (struct :`R` 1.0 :`B` 0.363356 :`A` 1.0)))

(fn `UserConstructionScript`)